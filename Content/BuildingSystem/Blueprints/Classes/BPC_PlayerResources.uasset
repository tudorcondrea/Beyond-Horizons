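; Player component that manages the resources used by the building system and tracks which one is currently selected.
; On initialization it has the player's main widget generate a widget per resource, fills in amounts and highlights the selection.
; Cycling steps through the resource map's keys with wrap-around, then updates the HUD and notifies the building manager.
; Amount refreshes notify the building manager only for the selected resource in a specific player state.
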(event Custom|OnResourceSwitch
  (Default|OnResourceChanged (Variables|/Game/FirstPersonBP/Blueprints/FirstPersonCharacter.FirstPersonCharacter_C|GetBPC_Building_Manager (Variables|Default|GetPlayerRef))))

(event Custom|InitializeManager
  (params (Player :type First%20Person%20Character%20Object%20Reference))
  (Utilities|IsValid Player
    (:Is%20Valid
      (Variables|Default|SetPlayerRef Player)
      (Variables|Default|SetInitialized? true)
      (bind _createdwidgets (Default|GenerateResourceWidget (Variables|/Game/FirstPersonBP/Blueprints/FirstPersonCharacter.FirstPersonCharacter_C|GetMain%20Widget (Variables|Default|GetPlayerRef)) self))
      (Variables|Default|SetResourceWidgets _createdwidgets)
      (bind _keys (Utilities|Map|Keys (Variables|Default|GetResources)))
      (for _array_element _keys
        (CallFunction|UpdateResourceDisplay _array_element))
      (CallFunction|SelectCurrentResource))))

(event EventUpdateResourceDisplay
  (params (Resource :type BP%20Master%20Resource%20Class%20Reference))
  (bind (_success_ _widget) (CallFunction|GetWidgetforResource Resource))
  (if (Variables|Default|GetInitialized?)
    (if _success_
      (Rendering|Components|TextRender|SetText (Variables|/Game/BuildingSystem/Widgets/W_Resources.W_Resources_C|GetAmount _widget) (Utilities|Text|ToText(Integer) (CallFunction|GetResource Resource) false false))
      (if (and (== (CallFunction|GetSelectedResource) Resource) (Utilities|Enum|Equal(Enum) (Variables|/Game/FirstPersonBP/Blueprints/FirstPersonCharacter.FirstPersonCharacter_C|GetStates (Variables|Default|GetPlayerRef)) "NewEnumerator1"))
        (Default|UpdateCurrentResource (Variables|/Game/FirstPersonBP/Blueprints/FirstPersonCharacter.FirstPersonCharacter_C|GetMain%20Widget (Variables|Default|GetPlayerRef)) self)
        (Default|OnResourceValueModify (Variables|/Game/FirstPersonBP/Blueprints/FirstPersonCharacter.FirstPersonCharacter_C|GetBPC_Building_Manager (Variables|Default|GetPlayerRef)) Resource)))))

(fn GetSelectedIndex
  (return (Variables|Default|GetSelectedResourceIndex)))

(fn GetSelectedResource
  (bind _keys (Utilities|Map|Keys (Variables|Default|GetResources)))
  (return (Utilities|Array|Get(acopy) _keys (Variables|Default|GetSelectedResourceIndex))))

(fn GetWidgetforResource
  (params (Resource :type BP%20Master%20Resource%20Class%20Reference))
  (bind _array_element (Utilities|Array|ForEachLoopwithBreak (Variables|Default|GetResourceWidgets) :!label _label)
    (:LoopBody
      (if (== (Variables|/Game/BuildingSystem/Widgets/W_Resources.W_Resources_C|GetResource _array_element) Resource)
        (LocalVariables|SetLocalFoundWidget _array_element)
        (goto _label Break)))
    (:Completed
      (Utilities|IsValid (LocalVariables|GetLocalFoundWidget)
        (:Is%20Valid
          (return true (LocalVariables|GetLocalFoundWidget)))
        (:Is%20Not%20Valid
          (return false 0))))))

(fn GetCurrentlySelectedWidget
  (return (.widget (CallFunction|GetWidgetforResource (CallFunction|GetSelectedResource)))))

(fn SelectCurrentResource
  (Default|SelectResource (CallFunction|GetCurrentlySelectedWidget) true false)
  (return))

(fn SelectNextResource
  (Default|SelectResource (CallFunction|GetCurrentlySelectedWidget) false false)
  (bind _keys (Utilities|Map|Keys (Variables|Default|GetResources)))
  (Variables|Default|SetSelectedResourceIndex (Math|Integer|SelectInt (+ (Variables|Default|GetSelectedResourceIndex) 1) 0 (< (Variables|Default|GetSelectedResourceIndex) (Utilities|Array|LastIndex _keys))))
  (CallFunction|SelectCurrentResource)
  (Default|UpdateCurrentResource (Variables|/Game/FirstPersonBP/Blueprints/FirstPersonCharacter.FirstPersonCharacter_C|GetMain%20Widget (Variables|Default|GetPlayerRef)) self)
  (CallFunction|OnResourceSwitch))