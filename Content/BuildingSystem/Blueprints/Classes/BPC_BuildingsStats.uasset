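; Actor component that manages a building's stats, including health, in the building system.
; InitializeManager caches a valid owning Building and runs stat setup.
; Stats live in an enum-keyed map of min, current and max values; changing a maximum re-clamps the current value and optionally fires UpdateStat.
; UpdateStat checks for health changes while the building is in player sight, but that branch is empty.
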(event Custom|InitializeManager
  (params (Building :type BP%20Master%20Building%20Object%20Reference))
  (Utilities|IsValid Building
    (:Is%20Valid
      (Variables|Default|SetBuilding Building)
      (CallFunction|SetUpStats))))

(event EventUpdateStat
  (params (Stat :type E_Stats%20Enum :default "NewEnumerator0"))
  (if (and (Utilities|Enum|Equal(Enum) Stat "NewEnumerator2") (Variables|/Game/BuildingSystem/Blueprints/Classes/BP_Master_Building.BP_Master_Building_C|GetInPlayerSight (Variables|Default|GetBuilding)))
    _))

(fn GetMaxHealth
  (return (.MaxValue (Utilities|Struct|BreakS_statValue (.Stat%20Value (CallFunction|GetStat "NewEnumerator2"))))))

(fn SetMaxStatValue
  (params (Stat :type E_Stats%20Enum :default "NewEnumerator0") (NewValue :type Integer) (Update? :type Boolean))
  (LocalVariables|SetLocalStat Stat)
  (LocalVariables|SetLocalValue NewValue)
  (LocalVariables|SetLocalUpdate Update?)
  (bind _keys (Utilities|Map|Keys (Variables|Default|GetStats)))
  (if (and (Utilities|Array|ContainsItem _keys (LocalVariables|GetLocalStat)) (Utilities|Enum|NotEqual(Enum) (LocalVariables|GetLocalStat) "NewEnumerator0"))
    (Utilities|Map|Add (Variables|Default|GetStats) (LocalVariables|GetLocalStat) (Utilities|Struct|MakeS_statValue (.MinValue (Utilities|Struct|BreakS_statValue (.Stat%20Value (CallFunction|GetStat (LocalVariables|GetLocalStat))))) (Math|Integer|Clamp(Integer) (.Current%20Value (CallFunction|GetStat (LocalVariables|GetLocalStat))) (.MinValue (Utilities|Struct|BreakS_statValue (.Stat%20Value (CallFunction|GetStat (LocalVariables|GetLocalStat))))) (LocalVariables|GetLocalValue)) (LocalVariables|GetLocalValue)))
    (if (LocalVariables|GetLocalUpdate)
      (CallFunction|UpdateStat (LocalVariables|GetLocalStat))
      (return)
      (else
        (return)))
    (else
      (return))))