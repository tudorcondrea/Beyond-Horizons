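; Component that manages crafting resource quantities for the building system in a CraftingResources map.
; GetResourceAmount returns the stored quantity, or -1 when the resource is missing.
; AddResource and RemoveResource ignore non-positive amounts and write back clamped quantities, though newly added entries are unclamped and removal skips missing resources.
; UpdateResourcesDisplay is an empty stub that none of these functions call.
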(fn GetResourceAmount
  (params (Resource :type E_CraftingMaterials%20Enum :default "NewEnumerator0"))
  (bind _craftingresources (Variables|Default|GetCraftingResources))
  (bind (_value _returnvalue) (Utilities|Map|Find _craftingresources Resource))
  (if _returnvalue
    (return (.quantity _value))
    (else
      (return -1))))

(fn AddResource
  (params (Resource :type E_CraftingMaterials%20Enum :default "NewEnumerator0") (Amount :type Integer))
  (bind _craftingresources (Variables|Default|GetCraftingResources))
  (LocalVariables|SetLocal%20Resource Resource)
  (LocalVariables|SetLocal%20Amount Amount)
  (if (> Amount 0)
    (if (.ReturnValue (Utilities|Map|Find (Variables|Default|GetCraftingResources) (LocalVariables|GetLocal%20Resource)))
      (Utilities|Map|Add _craftingresources (LocalVariables|GetLocal%20Resource) (Utilities|Struct|MakeS_CraftingResourceData (Math|Integer|Clamp(Integer) (+ (.quantity (.Value (Utilities|Map|Find (Variables|Default|GetCraftingResources) (LocalVariables|GetLocal%20Resource)))) (LocalVariables|GetLocal%20Amount)) 0 999) 0))
      (else
        (Utilities|Map|Add _craftingresources (LocalVariables|GetLocal%20Resource) (Utilities|Struct|MakeS_CraftingResourceData (LocalVariables|GetLocal%20Amount) 0))))
    (return)
    (else
      (return))))

(fn RemoveResource
  (params (Resource :type E_CraftingMaterials%20Enum :default "NewEnumerator0") (Amount :type Integer))
  (LocalVariables|SetLocalResource Resource)
  (LocalVariables|SetLocal%20Amount Amount)
  (if (> Amount 0)
    (if (.ReturnValue (Utilities|Map|Find (Variables|Default|GetCraftingResources) (LocalVariables|GetLocalResource)))
      (Utilities|Map|Add (Variables|Default|GetCraftingResources) (LocalVariables|GetLocalResource) (Utilities|Struct|MakeS_CraftingResourceData (Math|Integer|Clamp(Integer) (- (.quantity (.Value (Utilities|Map|Find (Variables|Default|GetCraftingResources) (LocalVariables|GetLocalResource)))) (LocalVariables|GetLocal%20Amount)) 0 999) 0))
      (return)
      (else
        (return)))
    (else
      (return))))

(fn UpdateResourcesDisplay
  (params (Resource :type E_CraftingMaterials%20Enum :default "NewEnumerator0")))