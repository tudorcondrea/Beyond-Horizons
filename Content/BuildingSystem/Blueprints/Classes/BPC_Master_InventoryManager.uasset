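; Inventory manager component in the building system that opens and closes the inventory UI.
; ToggleInventory creates a W_InventoryWidget linked to itself and adds it auto-sized and center-aligned to the HUD canvas of the FirstPersonCharacter's main widget.
; If the widget already exists, it removes and clears it instead.
; Input switches to UI-only with a locked mouse while open, and back to game-only on close.
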(event EventBeginPlay)

(event EventTick
  (params (DeltaSeconds :type Float%20%28single-precision%29)))

(fn ToggleInventory
  (Variables|Default|GetInventoryWidget
    (:then
      (Widget|RemovefromParent (Variables|Default|GetInventoryWidget))
      (Variables|Default|SetInventoryWidget 0)
      (Input|SetInputModeGameOnly (Game|GetPlayerController 0)))
    (:else
      (bind _returnvalue (UserInterface|CreateWidget "/Game/BuildingSystem/Widgets/W_InventoryWidget.W_InventoryWidget_C" 0 self))
      (Variables|Default|SetInventoryWidget _returnvalue)
      (bind _asfirst_person_character (Utilities|Casting|CastToFirstPersonCharacter (Game|GetPlayerCharacter 0)))
      (bind _returnvalue_2 (Class|CanvasPanel|AddChildtoCanvas (Variables|/Game/BuildingSystem/Widgets/W_Main.W_Main_C|GetHudCanvas (Variables|/Game/FirstPersonBP/Blueprints/FirstPersonCharacter.FirstPersonCharacter_C|GetMain%20Widget _asfirst_person_character)) (Variables|Default|GetInventoryWidget)))
      (Class|CanvasPanelSlot|SetAutoSize _returnvalue_2 true)
      (Class|CanvasPanelSlot|SetAlignment _returnvalue_2 "(X=0.500000,Y=0.500000)")
      (Class|CanvasPanelSlot|SetAnchors _returnvalue_2 (Variables|Default|GetAnchors))
      (Input|SetInputModeUIOnly (Game|GetPlayerController 0) (Variables|Default|GetInventoryWidget) "LockAlways"))))