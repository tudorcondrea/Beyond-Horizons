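; Player stats component that displays the player's oxygen level and heart rate on the main HUD widget.
; InitializeManager caches the player and sets up the stats, and OnStatSetUp initializes a bar for each key in the Stats map.
; UpdateStat pushes a stat's current value to its bar, with GetBarForStat selecting the matching widget through the player reference.
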(event Custom|InitializeManager
  (params (Player :type First%20Person%20Character%20Object%20Reference))
  (Variables|Default|SetPlayerRef Player)
  (CallFunction|SetUpStats))

(event EventOnStatSetUp
  (bind _keys (Utilities|Map|Keys (Variables|Default|GetStats)))
  (for _array_element _keys
    (Default|InitializeBar (CallFunction|GetBarforStat _array_element) (.Stat%20Value (CallFunction|GetStat _array_element)))))

(event EventUpdateStat
  (params (Stat :type E_Stats%20Enum :default "NewEnumerator0"))
  (Default|UpdateStat (CallFunction|GetBarforStat Stat) (.Current%20Value (CallFunction|GetStat Stat))))

(fn GetBarforStat
  (params (Stat :type E_Stats%20Enum :default "NewEnumerator0"))
  (bind _playerref (Variables|Default|GetPlayerRef))
  (bind _main_widget (Variables|/Game/FirstPersonBP/Blueprints/FirstPersonCharacter.FirstPersonCharacter_C|GetMain%20Widget _playerref))
  (return (Utilities|Select :Index Stat :NewEnumerator0 0 :NewEnumerator1 (Variables|/Game/BuildingSystem/Widgets/W_Main.W_Main_C|GetOxygenLevelWidget _main_widget) :NewEnumerator2 (Variables|/Game/BuildingSystem/Widgets/W_Main.W_Main_C|GetHeartRateWidget _main_widget))))