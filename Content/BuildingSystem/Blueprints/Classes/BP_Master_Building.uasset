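; Base building actor for the building system, starting as a placement ghost tinted by the selected resource, with a widget showing that resource's version info.
; Overlapping an already built building hides the ghost and widget.
; On build, it turns solid, takes the resource's material and removes the widget.
; A looping timer then raises a stat in the stats component toward max health over that resource version's build time.
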(event OnComponentBeginOverlap(Box)
  (params (OverlappedComponent :type Primitive%20Component%20Object%20Reference) (OtherActor :type Actor%20Object%20Reference) (OtherComp :type Primitive%20Component%20Object%20Reference) (OtherBodyIndex :type Integer) (bFromSweep :type Boolean) (SweepResult :type Hit%20Result%20Structure%20%28by%20ref%29))
  (if (!= OtherActor self)
    (Utilities|Casting|CastToStaticMeshComponent OtherComp)
    (bind _asbp_master_building (Utilities|Casting|CastToBP_Master_Building OtherActor))
    (if (Variables|BP_Master_Building_C|GetBuild? _asbp_master_building)
      (Utilities|Set|Add (Variables|Default|GetOverlappingBuilding) _asbp_master_building)
      (if (not (Variables|Default|GetOverlapping?))
        (CallFunction|OnOverlappingBegin)))))

(event OnComponentEndOverlap(Box)
  (params (OverlappedComponent :type Primitive%20Component%20Object%20Reference) (OtherActor :type Actor%20Object%20Reference) (OtherComp :type Primitive%20Component%20Object%20Reference) (OtherBodyIndex :type Integer))
  (bind _overlappingbuilding (Variables|Default|GetOverlappingBuilding))
  (if (!= OtherActor self)
    (Utilities|Casting|CastToStaticMeshComponent OtherComp)
    (bind _asbp_master_building (Utilities|Casting|CastToBP_Master_Building OtherActor))
    (if (Utilities|Set|Contains (Variables|Default|GetOverlappingBuilding) _asbp_master_building)
      (Utilities|Set|Remove _overlappingbuilding _asbp_master_building)
      (bind _result (Utilities|Set|ToArray _overlappingbuilding))
      (if (<= (Utilities|Array|Length _result) 0)
        (CallFunction|OnOverlappingEnd)))))

(event Custom|SetCanBeBuilt
  (params (NewValue :type Boolean))
  (bind _output_get (Variables|Default|SetCanBeBuilt? NewValue))
  (Default|SetCanbeBuilt (Variables|Default|GetBuildWidgetRef) _output_get))

(event Custom|OnBuild
  (params (NewParam :type BP%20Master%20Resource%20Class%20Reference))
  (bind _bpc_buildingsstats (Variables|Default|GetBPC_BuildingsStats))
  (bind _resourceversions (Variables|Default|GetResourceVersions))
  (bind _buildingmesh (Variables|Default|GetBuildingMesh))
  (bind _value (Utilities|Map|Find _resourceversions NewParam))
  (bind (_requiredamount _buildingtime _maxhealth) (Utilities|Struct|BreakS_BuildingResourceVersion _value))
  (if (Utilities|IsValidClass NewParam)
    (Variables|Default|SetBuild? true)
    (Collision|SetCollisionResponsetoAllChannels _buildingmesh "ECR_Block")
    (Rendering|Material|SetMaterial _buildingmesh 0 (Utilities|Struct|BreakS_ResourceData (Utilities|GetClassDefaults NewParam)))
    (Components|DestroyComponent (Variables|Default|GetBuildWidget))
    (Default|SetMaxStatValue _bpc_buildingsstats "NewEnumerator0" _maxhealth false)
    (Default|SetStat _bpc_buildingsstats "NewEnumerator0" 0 false)
    (Variables|Default|SetBuildingTime _buildingtime)
    (bind _returnvalue (Utilities|Time|SetTimerbyEvent (delegate Custom|BuildingTick) (Variables|Default|GetTimer) true))
    (Variables|Default|SetBuildingTimerHandle _returnvalue)
    (Utilities|FlowControl|Delay (+ (Variables|Default|GetBuildingTime) (Variables|Default|GetTimer)))
    (CallFunction|BuildingEnd)))

(event Custom|OnOverlappingEnd
  (Variables|Default|SetOverlapping? false)
  (Rendering|SetVisibility (Variables|Default|GetBuildWidget) true false)
  (Rendering|SetVisibility (Variables|Default|GetBuildingMesh) true false))

(event Custom|BuildingTick
  (bind _bpc_buildingsstats (Variables|Default|GetBPC_BuildingsStats))
  (bind _maxhealth (Default|GetMaxHealth _bpc_buildingsstats))
  (Default|ModifyStat _bpc_buildingsstats "NewEnumerator2" (Math|Float|Ceil (/ (Math|Conversions|ToFloat(Integer) _maxhealth) (Math|Conversions|ToFloat(Integer) (Math|Float|Floor (/ (Variables|Default|GetBuildingTime) (Variables|Default|GetTimer)))))))
  (if (== (.Current%20Value (Default|GetStat _bpc_buildingsstats "NewEnumerator2")) _maxhealth)
    (CallFunction|BuildingEnd)))

(event Custom|BuildingEnd
  (if (Utilities|Time|IsValidTimerHandle (Variables|Default|GetBuildingTimerHandle))
    (Utilities|Time|ClearandInvalidateTimerbyHandle (Variables|Default|GetBuildingTimerHandle))))

(event Custom|OnEnterPlayerSight
  (Variables|Default|SetInPlayerSight true)
  (if (Variables|Default|GetBuild?)
    _))

(event Custom|OnLeavePlayerSight
  (Variables|Default|SetInPlayerSight false)
  (if (Variables|Default|GetBuild?)
    _))

(event Custom|OnOverlappingBegin
  (Variables|Default|SetOverlapping? true)
  (Rendering|SetVisibility (Variables|Default|GetBuildWidget) false false)
  (Rendering|SetVisibility (Variables|Default|GetBuildingMesh) false false))

(event EventBeginPlay
  (bind _buildingmesh (Variables|Default|GetBuildingMesh))
  (bind _returnvalue (Rendering|Material|CreateDynamicMaterialInstance _buildingmesh 0 (Rendering|Material|GetMaterial _buildingmesh 0) "None" :!class /Script/Engine.PrimitiveComponent))
  (Variables|Default|SetDynamicMaterial _returnvalue)
  (CallFunction|UpdateGhostMaterial)
  (bind _asw_build_widget (Utilities|Casting|CastToW_BuildWidget (UserInterface|GetUserWidgetObject (Variables|Default|GetBuildWidget))))
  (bind _output_get (Variables|Default|SetBuildWidgetRef _asw_build_widget))
  (Default|Update _output_get (.Value (Utilities|Map|Find (Variables|Default|GetResourceVersions) (Variables|Default|GetResource))) (Variables|Default|GetResource))
  (Default|InitializeManager (Variables|Default|GetBPC_BuildingsStats) self)
  (Rendering|SetVisibility (Variables|Default|GetBuildWidget) true false))

(fn ConstructionScript)

(fn UpdateGhostMaterial
  (Rendering|Material|SetVectorParameterValue (Variables|Default|GetDynamicMaterial) "Color" (Utilities|Struct|BreakS_ResourceData (Utilities|GetClassDefaults (Variables|Default|GetResource))) :!class /Script/Engine.MaterialInstanceDynamic)
  (return))

(fn ChangeResource
  (params (NewResource :type BP%20Master%20Resource%20Class%20Reference))
  (if (and (Utilities|IsValidClass NewResource) (!= NewResource (Variables|Default|GetResource)))
    (Variables|Default|SetResource NewResource)
    (CallFunction|UpdateGhostMaterial)
    (Default|Update (Variables|Default|GetBuildWidgetRef) (.Value (Utilities|Map|Find (Variables|Default|GetResourceVersions) (Variables|Default|GetResource))) (Variables|Default|GetResource))
    (return)
    (else
      (return))))