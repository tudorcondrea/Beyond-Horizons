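; BP_MasterResourceNodes is a damageable resource node in the building system that yields resources to the player who hits it.
; On BeginPlay it snapshots its ResourceManager contents and initializes the health stat in BPCBuildingsStats.
; Player damage moves a share of each original resource, proportional to health actually lost, into the player's resource component, clamped between one and the remaining stock.
; After a player's hit depletes health, the node is destroyed.
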(event EventBeginPlay
  (bind _bpc_buildingsstats (Variables|Default|GetBPC_BuildingsStats))
  (bind _maxhealth (Variables|Default|GetMaxHealth))
  (CallFunction|SetUpOriginalResources)
  (Default|SetMaxStatValue _bpc_buildingsstats "NewEnumerator2" _maxhealth false)
  (Default|SetStat _bpc_buildingsstats "NewEnumerator2" _maxhealth false)
  (Default|InitializeManager (Variables|Default|GetBPC_BuildingsStats) self))

(event Game|Damage|EventAnyDamage
  (params (Damage :type Float%20%28single-precision%29) (DamageType :type Damage%20Type%20Object%20Reference) (InstigatedBy :type Controller%20Object%20Reference) (DamageCauser :type Actor%20Object%20Reference))
  (bind _bpc_buildingsstats (Variables|Default|GetBPC_BuildingsStats))
  (bind _current_value (Default|GetStat _bpc_buildingsstats "NewEnumerator2"))
  (Variables|Default|SetHealthBefore _current_value)
  (Default|ModifyStat (Variables|Default|GetBPC_BuildingsStats) "NewEnumerator2" (Math|Float|Round (* -1 Damage)))
  (Variables|Default|SetHealthAfter _current_value)
  (bind _asfirst_person_character (Utilities|Casting|CastToFirstPersonCharacter DamageCauser))
  (CallFunction|GiveResourcestoPlayer _asfirst_person_character (- (Variables|Default|GetHealthBefore) (Variables|Default|GetHealthAfter)))
  (if (<= (.Current%20Value (Default|GetStat (Variables|Default|GetBPC_BuildingsStats) "NewEnumerator2")) 0)
    (CallFunction|DestroyBuilding)))

(fn ConstructionScript
  (|CallParentFunction))

(fn SetUpOriginalResources
  (bind _resourcemanager (Variables|Default|GetResourceManager))
  (bind _keys (Utilities|Map|Keys (Variables|/Game/BuildingSystem/Blueprints/Classes/BPC_Master_ResourceManager.BPC_Master_ResourceManager_C|GetResources _resourcemanager)))
  (for _array_element _keys
    (Utilities|Map|Add (Variables|Default|GetOriginalResources) _array_element (Default|GetResource _resourcemanager _array_element))))

(fn GiveResourcestoPlayer
  (params (Player :type First%20Person%20Character%20Object%20Reference) (DealtDamage :type Integer))
  (if (> DealtDamage 0)
    (LocalVariables|SetLocalPercentage (/ (Math|Conversions|ToFloat(Integer) DealtDamage) (Math|Conversions|ToFloat(Integer) (Default|GetMaxHealth (Variables|Default|GetBPC_BuildingsStats)))))
    (bind _keys (Utilities|Map|Keys (Variables|/Game/BuildingSystem/Blueprints/Classes/BPC_Master_ResourceManager.BPC_Master_ResourceManager_C|GetResources (Variables|Default|GetResourceManager))))
    (for _array_element _keys
      (if (> (Default|GetResource (Variables|Default|GetResourceManager) _array_element) 0)
        (bind _output_get (LocalVariables|SetLocalAmount (Math|Integer|Clamp(Integer) (Math|Float|Ceil (* (.Value (Utilities|Map|Find (Variables|Default|GetOriginalResources) _array_element)) (LocalVariables|GetLocalPercentage))) 1 (Default|GetResource (Variables|Default|GetResourceManager) _array_element))))
        (Default|RemoveResource (Variables|Default|GetResourceManager) _array_element _output_get)
        (Default|AddResource (Variables|/Game/FirstPersonBP/Blueprints/FirstPersonCharacter.FirstPersonCharacter_C|GetBPC_PlayerResources Player) _array_element _output_get)))
    (else
      (return))))